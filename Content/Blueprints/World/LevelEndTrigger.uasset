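; LevelEndTrigger is a world actor that marks the exit of a level and reports success when the player reaches it.
; On BeginPlay it casts the game mode to BankMode, caches it, and registers itself as that mode's ExitDoor.
; When player 0's pawn begins overlapping it, it calls NoteLevelSuccess on BankMode, leaving the end-of-level handling to the game mode.
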(event EventBeginPlay
  (bind _asbank_mode (Utilities|Casting|CastToBankMode (Game|GetGameMode)))
  (bind _output_get (Variables|Default|SetBankMode _asbank_mode))
  (Variables|/Game/Blueprints/BankMode.BankMode_C|SetExitDoor _output_get self))

(event Collision|EventActorBeginOverlap
  (params (OtherActor :type Actor%20Object%20Reference))
  (if (and (Utilities|IsValid OtherActor) (== OtherActor (Game|Player|GetPlayerPawn 0)))
    (Default|NoteLevelSuccess (Variables|Default|GetBankMode))))

(fn ConstructionScript)