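; BankMode is a mode Blueprint that sets up the camera, mouse input, HUD and cursor-driven aiming reticle.
; BeginPlay switches the view to the level's FollowCamera, sets game-and-UI input, finds the Reticle actor and adds the HUD widget.
; Each tick, an under-cursor trace against one object type moves the reticle in XY at fixed height and stores CursorTargetLocation, hiding it on a miss.
; NoteLevelSuccess is an empty stub.
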(event EventBeginPlay
  (bind _returnvalue (Game|GetPlayerController 0))
  (Utilities|FlowControl|Sequence
    (:then_0
      (bind _outactors (Actor|GetAllActorsOfClass "/Game/Blueprints/FollowCamera.FollowCamera_C"))
      (Utilities|IsValid (Utilities|Array|Get(acopy) _outactors)
        (:Is%20Valid
          (Game|Player|SetViewTargetwithBlend (Game|GetPlayerController 0) (Utilities|Array|Get(acopy) _outactors) 0.0 "VTBlend_Linear" 0.0 false))))
    (:then_1
      (Input|EnableInput _returnvalue)
      (Class|WidgetBlueprintLibrary|SetFocustoGameViewport)
      (Input|SetInputModeGameandUI _returnvalue 0 "LockOnCapture" false))
    (:then_2
      (bind _outactors_2 (Actor|GetAllActorsOfClass "/Game/Blueprints/Reticle.Reticle_C"))
      (Variables|Default|SetReticle (Utilities|Array|Get(acopy) _outactors_2)))
    (:then_3
      (bind _returnvalue_2 (UserInterface|CreateWidget "/Game/Blueprints/UI/HUD.HUD_C" (Game|GetPlayerController 0)))
      (bind _output_get (Variables|Default|SetHUDWidget _returnvalue_2))
      (UserInterface|Viewport|AddtoViewport _output_get 0))))

(event EventTick
  (params (DeltaSeconds :type Float%20%28single-precision%29))
  (CallFunction|UpdateCursorAim))

(fn ConstructionScript)

(fn UpdateCursorAim
  (bind _returnvalue (Game|GetPlayerController 0))
  (bind _array (Utilities|Array|MakeArray "ObjectTypeQuery10"))
  (bind _reticle (Variables|Default|GetReticle))
  (bind _returnvalue_2 (Transformation|GetActorLocation _reticle))
  (bind _hitresult (Class|PlayerController|GetHitResultUnderCursorforObjects _returnvalue _array true))
  (bind (_bblockinghit _binitialoverlap _time _distance _location) (Collision|BreakHitResult _hitresult))
  (bind (_x _y) (Math|Vector|BreakVector _location))
  (bind _returnvalue_3 (Math|Vector|MakeVector _x _y (.z _returnvalue_2)))
  (if _bblockinghit
    (Rendering|SetActorHiddenInGame _reticle false)
    (Transformation|SetActorLocation _reticle _returnvalue_3 false true)
    (Variables|Default|SetCursorTargetLocation _returnvalue_3)
    (else
      (Rendering|SetActorHiddenInGame (Variables|Default|GetReticle) true))))

(fn NoteLevelSuccess)