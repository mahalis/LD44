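; Rusher enemy that wanders the navmesh, chases the player once noticed within its alert radius, and stops to charge an attack at close range.
; Tick runs wander or chase logic using PlayerAwarenessComponent, switching between following the player and their last seen location before giving up.
; Function-name timers drive wandering, attack charge and cooldown; the attack itself only prints.
; When DamageHandlingComponent's damage handler returns true, movement and timers stop.
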(event EventBeginPlay
  (CallFunction|StartWandering)
  (bind _returnvalue (Rendering|Material|CreateDynamicMaterialInstance 0 "None" :!class /Script/Engine.KismetMaterialLibrary))
  (Variables|Default|SetLegMovementMaterial _returnvalue))

(event Collision|EventActorBeginOverlap
  (params (OtherActor :type Actor%20Object%20Reference)))

(event EventTick
  (params (DeltaSeconds :type Float%20%28single-precision%29))
  (if (Variables|/Game/Blueprints/Enemy/DamageHandlingComponent.DamageHandlingComponent_C|GetIsAlive (Variables|Default|GetDamageHandlingComponent))
    (if (Variables|Behavior|GetIsChasing)
      (CallFunction|ThinkChasing)
      (else
        (CallFunction|ThinkWandering)))))

(event Game|Damage|EventAnyDamage
  (params (Damage :type Float%20%28single-precision%29) (DamageType :type Damage%20Type%20Object%20Reference) (InstigatedBy :type Controller%20Object%20Reference) (DamageCauser :type Actor%20Object%20Reference))
  (bind _died (Default|HandleDamageTaken (Variables|Default|GetDamageHandlingComponent) Damage))
  (if _died
    (AI|Navigation|StopMovement (AI|GetAIController self))
    (Utilities|FlowControl|Sequence
      (:then_0
        (Utilities|Time|ClearTimerbyFunctionName 0 "PickNewWanderLocation"))
      (:then_1
        (Utilities|Time|ClearTimerbyFunctionName 0 "DoAttack"))
      (:then_2
        (Utilities|Time|ClearTimerbyFunctionName 0 "ResetAfterAttack")))))

(fn ConstructionScript)

(fn PickNewWanderLocation
  (bind _returnvalue (Pawn|GetNavAgentLocation))
  (bind (_randomlocation _returnvalue_2) (AI|Navigation|GetRandomReachablePointinRadius _returnvalue 1e+03 0 "/Script/NavigationSystem.RecastFilter_UseDefaultArea"))
  (if _returnvalue_2
    (AI|Navigation|MovetoLocation (AI|GetAIController self) _randomlocation 5.0 true true false true 0)))

(fn StartChasing
  (Utilities|Time|ClearTimerbyFunctionName 0 "PickNewWanderLocation")
  (Variables|Behavior|SetIsChasing true)
  (AI|Navigation|MovetoActor (AI|GetAIController self) (Game|Player|GetPlayerPawn 0) 5.0 true true true 0)
  (Variables|Default|SetIsChasingPlayerCurrentLocation true)
  (Development|PrintString "started chasing" true true "(R=0.591172,G=0.859375,B=0.030666,A=1.000000)"))

(fn StartWandering
  (Variables|Behavior|SetIsChasing false)
  (Utilities|Time|SetTimerbyFunctionName 0 "PickNewWanderLocation" 1.0 true)
  (CallFunction|PickNewWanderLocation)
  (Development|PrintString "started wandering" true true "(R=0.195759,G=0.390625,B=0.024211,A=1.000000)"))

(fn UpdateChaseType
  (bind _self self)
  (bind _returnvalue (AI|GetAIController _self))
  (if (Math|Boolean|NotEqual(Boolean) (< (Utilities|Time|GetGameTimeinSeconds) (+ (Variables|/Game/Blueprints/Enemy/PlayerAwarenessComponent.PlayerAwarenessComponent_C|GetLastSeenPlayerTime (Variables|Default|GetPlayerAwarenessComponent)) 0.1)) (Variables|Default|GetIsChasingPlayerCurrentLocation)) ; yes - we need to change chase types
    (if (Variables|Default|GetIsChasingPlayerCurrentLocation)
      (Variables|Default|SetIsChasingPlayerCurrentLocation false)
      (AI|Navigation|MovetoLocation _returnvalue (Variables|/Game/Blueprints/Enemy/PlayerAwarenessComponent.PlayerAwarenessComponent_C|GetLastSeenPlayerLocation (Variables|Default|GetPlayerAwarenessComponent)) 5.0 true true true true 0)
      (Development|PrintString "lost sight of player, going to last location" true true "(R=0.195759,G=0.390625,B=0.024211,A=1.000000)")
      (else
        (Variables|Default|SetIsChasingPlayerCurrentLocation true)
        (AI|Navigation|MovetoActor _returnvalue (Game|Player|GetPlayerPawn 0) 5.0 true true true 0)
        (Development|PrintString "regained sight of player, following" true true "(R=0.195759,G=0.390625,B=0.024211,A=1.000000)")))))

(fn ThinkChasing
  (if (not (Variables|Attack|GetIsAttacking))
    (Default|Update (Variables|Default|GetPlayerAwarenessComponent))
    (CallFunction|UpdateChaseType)
    (CallFunction|StartChargingAttackifPossible)
    (if (and (> (Utilities|Time|GetGameTimeinSeconds) (+ (Variables|/Game/Blueprints/Enemy/PlayerAwarenessComponent.PlayerAwarenessComponent_C|GetLastSeenPlayerTime (Variables|Default|GetPlayerAwarenessComponent)) (Variables|Constants|GetGiveUpChaseDelay))) (Variables|Behavior|GetIsChasing)) ; is it time to give up?
      (CallFunction|StartWandering))))

(fn ThinkWandering
  (if (< (Math|Vector|Distance(Vector) (Transformation|GetActorLocation) (Transformation|GetActorLocation (Game|Player|GetPlayerPawn 0))) (Variables|Constants|GetAlertRadius))
    (bind _seen (Default|Update (Variables|Default|GetPlayerAwarenessComponent)))
    (if _seen
      (CallFunction|StartChasing))))

(fn StartChargingAttackifPossible
  (if (not (Variables|Attack|GetIsAttacking))
    (if (< (Math|Vector|Distance(Vector) (Transformation|GetActorLocation) (Transformation|GetActorLocation (Game|Player|GetPlayerPawn 0))) (Variables|Constants|GetAttackTriggerRadius))
      (Variables|Attack|SetIsAttacking true)
      (Utilities|FlowControl|Sequence
        (:then_0
          (Variables|Attack|SetAttackChargeStartTime (Utilities|Time|GetGameTimeinSeconds)))
        (:then_1
          (Utilities|Time|SetTimerbyFunctionName 0 "DoAttack" (Variables|Constants|GetAttackChargeDuration)))
        (:then_2
          (Development|PrintString "started charging pow"))
        (:then_3
          (AI|Navigation|StopMovement (AI|GetAIController self)))))))

(fn DoAttack
  (Development|PrintString "pow!!" true true "(R=0.000000,G=0.660000,B=1.000000,A=1.000000)" 0.5)
  (Utilities|Time|SetTimerbyFunctionName 0 "ResetAfterAttack" (Variables|Constants|GetPostAttackCooldownDuration)))

(fn ResetAfterAttack
  (Variables|Attack|SetIsAttacking false)
  (bind _seen (Default|Update (Variables|Default|GetPlayerAwarenessComponent)))
  (if _seen
    (CallFunction|StartChasing)
    (else
      (CallFunction|StartWandering))))