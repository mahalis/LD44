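; Base enemy Blueprint that tracks health and handles death for AI-controlled enemies.
; Health starts from StartingHealth on BeginPlay, and DecrementHealth subtracts damage, calling Die when it reaches zero and returning whether the hit was lethal.
; Die stops the AI controller's brain logic, while destruction is a separate FinishDying function, leaving room for a death sequence before removal.
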(event EventBeginPlay
  (Variables|Default|SetHealth (Variables|Default|GetStartingHealth)))

(event Collision|EventActorBeginOverlap
  (params (OtherActor :type Actor%20Object%20Reference)))

(event EventTick
  (params (DeltaSeconds :type Float%20%28single-precision%29)))

(fn ConstructionScript)

(fn Die
  (Variables|Default|SetHealth 0)
  (bind _asaicontroller (Utilities|Casting|CastToAIController (Pawn|GetController)))
  (AI|Logic|StopLogic (Variables|/Script/AIModule.AIController|GetBrainComponent _asaicontroller) "dying"))

(fn FinishDying
  (Actor|DestroyActor))

(fn DecrementHealth
  (params (Amount :type Integer))
  (if (<= (- (Variables|Default|GetHealth) Amount) 0) ; did this kill us?
    (CallFunction|Die)
    (return true)
    (else
      (Variables|Default|SetHealth (- (Variables|Default|GetHealth) Amount))
      (return false))))