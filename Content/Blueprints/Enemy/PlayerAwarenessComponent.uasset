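; Enemy actor component that tracks whether its owner has line of sight to the player.
; Update line-traces from the owner's location to a point slightly above the player pawn's location and checks whether the first hit is the player.
; On a hit it records the current game time and player position as last-seen data, and in either case returns whether the player is visible.
; Tick and BeginPlay are unused, so detection runs only when Update is called.
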(event EventBeginPlay)

(event EventTick
  (params (DeltaSeconds :type Float%20%28single-precision%29)))

(fn Update
  (bind _returnvalue (Game|Player|GetPlayerPawn 0))
  (bind _returnvalue_2 (Transformation|GetActorLocation _returnvalue))
  (bind _outhit (Collision|LineTraceByChannel (Transformation|GetActorLocation (Components|GetOwner)) (+ _returnvalue_2 "0, 0,30.000000") "TraceTypeQuery3" false 0 "None" true "(R=1.000000,G=0.000000,B=0.000000,A=1.000000)" "(R=0.000000,G=1.000000,B=0.000000,A=1.000000)" 1.0))
  (Utilities|FlowControl|Sequence
    (:then_0
      (if (== _returnvalue (.hitactor _outhit)) ; was it the player?
        (Variables|Default|SetLastSeenPlayerTime (Utilities|Time|GetGameTimeinSeconds))
        (Variables|Default|SetLastSeenPlayerLocation _returnvalue_2)))
    (:then_1
      (return (== _returnvalue (.hitactor _outhit))))))