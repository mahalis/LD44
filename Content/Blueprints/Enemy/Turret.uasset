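; Enemy turret actor that sweeps back and forth around the yaw it has at BeginPlay.
; Tick runs DoScan only once ReturnToScanningDelay has elapsed since LastSeenPlayerTime, which nothing in these graphs updates.
; DoScan eases rotation with RInterpTo toward HeadingRange either side of the initial heading, flipping IsRotatingRight when nearly there.
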(event EventBeginPlay
  (Variables|Aim|SetInitialHeading (.yaw (Transformation|GetActorRotation))))

(event Collision|EventActorBeginOverlap
  (params (OtherActor :type Actor%20Object%20Reference)))

(event EventTick
  (params (DeltaSeconds :type Float%20%28single-precision%29))
  (if (> (- (Utilities|Time|GetGameTimeinSeconds) (Variables|Behavior|GetLastSeenPlayerTime)) (Variables|Constants|GetReturnToScanningDelay)) ; have we not seen the player recently?
    (CallFunction|DoScan DeltaSeconds)))

(fn ConstructionScript)

(fn DoScan
  (params (DeltaTime :type Float%20%28single-precision%29))
  (bind _returnvalue (Transformation|GetActorRotation))
  (Transformation|SetActorRotation (Math|Interpolation|RInterpTo _returnvalue (Math|Rotator|MakeRotator 0.0 0.0 (+ (Variables|Aim|GetInitialHeading) (* (Math|Float|SelectFloat 1.0 -1.0 (Variables|Aim|GetIsRotatingRight)) (Variables|Aim|GetHeadingRange)))) DeltaTime 2.0))
  (if (< (Math|Float|Absolute(Float) (- (.Yaw (Math|Rotator|BreakRotator _returnvalue)) (+ (Variables|Aim|GetInitialHeading) (* (Math|Float|SelectFloat 1.0 -1.0 (Variables|Aim|GetIsRotatingRight)) (Variables|Aim|GetHeadingRange))))) 3.0) ; are we close enough to the target rotation?
    (Variables|Aim|SetIsRotatingRight (not (Variables|Aim|GetIsRotatingRight)))))