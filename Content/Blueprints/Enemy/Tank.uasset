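; Enemy tank that wanders the navmesh while its upper part spins.
; A looping timer picks random reachable points nearby and sends the AI controller there, facing the destination.
; Tick updates the player awareness component, but the upper part spins at a constant rate regardless, as the look-at-last-seen-position logic is disconnected.
; When the damage handling component returns true, movement and the wander timer stop.
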(event EventBeginPlay
  (Utilities|Time|SetTimerbyFunctionName 0 "PickNewWanderLocation" 2.0 true)
  (CallFunction|PickNewWanderLocation))

(event Collision|EventActorBeginOverlap
  (params (OtherActor :type Actor%20Object%20Reference)))

(event EventTick
  (params (DeltaSeconds :type Float%20%28single-precision%29))
  (bind _seen (Default|Update (Variables|Default|GetPlayerAwarenessComponent)))
  (CallFunction|UpdateUpperRotation _seen DeltaSeconds))

(event Game|Damage|EventAnyDamage
  (params (Damage :type Float%20%28single-precision%29) (DamageType :type Damage%20Type%20Object%20Reference) (InstigatedBy :type Controller%20Object%20Reference) (DamageCauser :type Actor%20Object%20Reference))
  (bind _died (Default|HandleDamageTaken (Variables|Default|GetDamageHandlingComponent) Damage))
  (if _died
    (AI|Navigation|StopMovement (AI|GetAIController self))
    (Utilities|Time|ClearTimerbyFunctionName 0 "PickNewWanderLocation")))

(fn ConstructionScript)

(fn PickNewWanderLocation
  (bind _returnvalue (Pawn|GetNavAgentLocation))
  (bind _self self)
  (bind (_randomlocation _returnvalue_2) (AI|Navigation|GetRandomReachablePointinRadius _returnvalue 1e+03 0 "/Script/NavigationSystem.RecastFilter_UseDefaultArea"))
  (bind _returnvalue_3 (AI|GetAIController _self))
  (if _returnvalue_2
    (bind _output_get (LocalVariables|SetNextPoint _randomlocation))
    (AI|Navigation|MovetoLocation _returnvalue_3 _output_get 5.0 true true false false 0)
    (Pawn|SetControlRotation _returnvalue_3 (Math|Rotator|FindLookatRotation _returnvalue _output_get))))

(fn UpdateUpperRotation
  (params (CanSeePlayer :type Boolean) (DeltaTime :type Float%20%28single-precision%29))
  (Transformation|AddLocalRotation (Variables|Default|GetUpper) (Math|Rotator|MakeRotator 0.0 0.0 (* DeltaTime 1.2e+02)) false false))