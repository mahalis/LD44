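; Behavior tree service that checks each tick whether the AI-controlled enemy has line of sight to the player.
; It line-traces on the Camera channel from slightly above the pawn toward player pawn 0, ignoring itself, and draws a debug point at the hit.
; A hit on the player writes the player's location, seen time and pawn to the blackboard; otherwise only the seen-player key is cleared, keeping the last known position and time.
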(event EventReceiveTickAI
  (params (OwnerController :type AI%20Controller%20Object%20Reference) (ControlledPawn :type Pawn%20Object%20Reference) (DeltaSeconds :type Float%20%28single-precision%29))
  (bind _returnvalue (Game|Player|GetPlayerPawn 0))
  (bind _returnvalue_2 (Transformation|GetActorLocation _returnvalue))
  (bind _outhit (Collision|LineTraceByChannel (+ (Transformation|GetActorLocation ControlledPawn) "0, 0,40.000000") (+ _returnvalue_2 "0, 0,20.000000") "TraceTypeQuery2" false (Utilities|Array|MakeArray ControlledPawn) "None"))
  (Rendering|Debug|DrawDebugPoint (.location _outhit) 2.0 "(R=0.115994,G=1.000000,B=0.684332,A=1.000000)" 0.1)
  (if (== _returnvalue (.hitactor _outhit))
    (AI|BehaviorTree|SetBlackboardValueasVector (Variables|Default|GetPlayerLocationKey) _returnvalue_2)
    (Class|BTFunctionLibrary|SetBlackboardValueasFloat (Variables|Default|GetPlayerSeenTimeKey) (Utilities|Time|GetTimeSeconds))
    (Class|BTFunctionLibrary|SetBlackboardValueasObject (Variables|Default|GetSeenPlayerKey) _returnvalue)
    (else
      (Class|BTFunctionLibrary|ClearBlackboardValue (Variables|Default|GetSeenPlayerKey)))))