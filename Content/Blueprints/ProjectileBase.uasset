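; Base projectile Blueprint that deals point damage and plays an impact effect when it hits.
; A hit on a damageable actor ends the flight immediately; other hits end it only if the projectile movement is not set to bounce.
; HandleFinalImpact deactivates the trail, hides the mesh, disables sphere collision, stops movement, spawns the impact system along the surface normal and applies damage, without destroying the actor.
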(event EventBeginPlay)

(event Collision|EventActorBeginOverlap
  (params (OtherActor :type Actor%20Object%20Reference)))

(event EventTick
  (params (DeltaSeconds :type Float%20%28single-precision%29)))

(event Collision|EventHit
  (params (MyComp :type Primitive%20Component%20Object%20Reference) (Other :type Actor%20Object%20Reference) (OtherComp :type Primitive%20Component%20Object%20Reference) (bSelfMoved :type Boolean) (HitLocation :type Vector :default "0, 0, 0") (HitNormal :type Vector :default "0, 0, 0") (NormalImpulse :type Vector :default "0, 0, 0") (Hit :type Hit%20Result%20Structure%20%28by%20ref%29))
  (if (Utilities|IsValid Other)
    (if (Variables|/Script/Engine.Actor|GetbCanBeDamaged Other)
      (CallFunction|HandleFinalImpact Hit :!label _label)
      (else
        (if (not (Variables|/Script/Engine.ProjectileMovementComponent|GetbShouldBounce (Variables|Default|GetProjectileMovement))) :!label _label_2
          (goto _label))))
    (else
      (goto _label_2))))

(fn ConstructionScript)

(fn HandleFinalImpact
  (params (HitResult :type Hit%20Result%20Structure))
  (bind (_bblockinghit _binitialoverlap _time _distance _location _impactpoint _normal _impactnormal _physmat _hitactor) (Collision|BreakHitResult HitResult))
  (Components|Activation|SetActive (Variables|Default|GetTrail) false false)
  (Rendering|SetVisibility (Variables|Default|GetMesh) false true)
  (Collision|SetCollisionEnabled (Variables|Default|GetSphere) "NoCollision")
  (Game|Components|ProjectileMovement|StopSimulating (Variables|Default|GetProjectileMovement) HitResult)
  (Niagara|SpawnSystematLocation (Variables|Default|GetImpactSystem) _impactpoint (Math|Rotator|MakeRotfromZ _impactnormal))
  (Game|Damage|ApplyPointDamage _hitactor (Variables|Default|GetDamageAmount) _impactnormal HitResult 0 self))