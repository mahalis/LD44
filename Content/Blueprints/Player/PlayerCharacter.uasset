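; Player character for a bank-themed game that moves on diagonal world axes, aims at the cursor and shoots coins.
; Each tick yaws the actor toward the cursor target location read from BankMode, then fires if input is held and the shared cooldown has elapsed.
; Alt fire takes priority over primary, spawning a several-coins projectile instead of a single coin, each with its own interval.
; Escape quits the game.
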(event EventBeginPlay
  (bind _asbank_mode (Utilities|Casting|CastToBankMode (Game|GetGameMode)))
  (Variables|Default|SetBankMode _asbank_mode))

(event Collision|EventActorBeginOverlap
  (params (OtherActor :type Actor%20Object%20Reference)))

(event EventTick
  (params (DeltaSeconds :type Float%20%28single-precision%29))
  (CallFunction|UpdateAim DeltaSeconds)
  (CallFunction|FireifDesired))

(event Game|Damage|EventAnyDamage
  (params (Damage :type Float%20%28single-precision%29) (DamageType :type Damage%20Type%20Object%20Reference) (InstigatedBy :type Controller%20Object%20Reference) (DamageCauser :type Actor%20Object%20Reference)))

(event Input|ActionEvents|InputActionFire
  (params (Key :type Key%20Structure))
  (:Pressed
    (Variables|Firing|SetWantsFire true))
  (:Released
    (Variables|Firing|SetWantsFire false)))

(event Input|ActionEvents|InputActionAltFire
  (params (Key :type Key%20Structure))
  (:Pressed
    (Variables|Firing|SetWantsAltFire true))
  (:Released
    (Variables|Firing|SetWantsAltFire false)))

(event Input|AxisEvents|InputAxisForward
  (params (AxisValue :type Float%20%28single-precision%29))
  (Class|PawnMovementComponent|AddInputVector (Variables|Character|GetCharacterMovement) (* "0.707100,0.707100, 0" AxisValue) false))

(event Input|AxisEvents|InputAxisRight
  (params (AxisValue :type Float%20%28single-precision%29))
  (Class|PawnMovementComponent|AddInputVector (Variables|Character|GetCharacterMovement) (* "-0.707100,0.707100, 0" AxisValue) false))

(event Input|KeyboardEvents|Escape
  (params (Key :type Key%20Structure))
  (:Pressed
    (Game|QuitGame (Game|GetPlayerController 0) "Quit" false)))

(fn ConstructionScript)

(fn FireifDesired
  (if (> (Utilities|Time|GetGameTimeinSeconds) (Variables|Firing|GetNextAllowedFireTime))
    (if (Variables|Firing|GetWantsAltFire)
      (CallFunction|DoAltFire)
      (elif (Variables|Firing|GetWantsFire)
        (CallFunction|DoPrimaryFire)))))

(fn DoPrimaryFire
  (Variables|Firing|SetNextAllowedFireTime (+ (Utilities|Time|GetGameTimeinSeconds) (Variables|Constants|GetPrimaryFireInterval)))
  (Game|SpawnActorfromClass "/Game/Blueprints/Player/CoinProjectile.CoinProjectile_C" (Transformation|GetWorldTransform (Variables|Default|GetCoinSpawnLocation)) "AlwaysSpawn" 0 self))

(fn DoAltFire
  (Variables|Firing|SetNextAllowedFireTime (+ (Utilities|Time|GetGameTimeinSeconds) (Variables|Constants|GetAltFireInterval)))
  (Game|SpawnActorfromClass "/Game/Blueprints/Player/SeveralCoinsProjectile.SeveralCoinsProjectile_C" (Transformation|GetWorldTransform (Variables|Default|GetCoinSpawnLocation)) "AlwaysSpawn" 0 self))

(fn UpdateAim
  (params (DeltaTime :type Float%20%28single-precision%29))
  (bind _returnvalue (Transformation|GetActorLocation))
  (bind _bankmode (Variables|Default|GetBankMode))
  (bind _cursortargetlocation (Variables|/Game/Blueprints/BankMode.BankMode_C|GetCursorTargetLocation _bankmode))
  (Transformation|SetActorRotation (Math|Rotator|MakeRotator 0.0 0.0 (- (.yaw (Math|Rotator|FindLookatRotation (Math|Vector|MakeVector (.x _returnvalue) (.y _returnvalue) 0.0) (Math|Vector|MakeVector (.x _cursortargetlocation) (.y _cursortargetlocation) 0.0))) 9e+01))))